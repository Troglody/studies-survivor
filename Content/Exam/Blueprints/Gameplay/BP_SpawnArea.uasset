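; Spawn area actor that periodically spawns a configurable actor class inside its Box, with waves arriving ever faster.
; Tick accumulates time and, at each interval, spawns a stack, then shortens the interval by 2 percent.
; Each stack has a random size and shares one random point in the inner half of the box at center height.
; Spawns face the player pawn's location, with collision adjustment separating them where possible.
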(event EventTick
  (params (DeltaSeconds :type Float%20%28single-precision%29))
  (bind _output_get (Variables|Gameplay|SetCurrentTime (+ DeltaSeconds (Variables|Gameplay|GetCurrentTime))))
  (if (>= _output_get (Variables|Gameplay|GetSpawnInterval))
    (Variables|Gameplay|SetCurrentTime (- (Variables|Gameplay|GetCurrentTime) (Variables|Gameplay|GetSpawnInterval)))
    (CallFunction|SpawnActor)
    (Variables|Gameplay|SetSpawnInterval (* (Variables|Gameplay|GetSpawnInterval) 0.98))))

(fn ConstructionScript)

(fn GetSpawnYaw
  (params (Origin :type Vector))
  (return (.yaw (Math|Rotator|FindLookatRotation Origin (Transformation|GetActorLocation (Game|Player|GetPlayerPawn 0))))))

(fn SpawnActor
  (LocalVariables|SetSpawnLocation (CallFunction|GetSpawnLocation))
  (for _index (range 1 (Math|Random|RandomIntegerinRange (Variables|Gameplay|GetMinSpawnStackSize) (Variables|Gameplay|GetMaxSpawnStackSize)))
    (Game|SpawnActorfromClass (Variables|Gameplay|GetSpawnedActor) (Math|Transform|MakeTransform (LocalVariables|GetSpawnLocation) (Math|Rotator|MakeRotator 0.0 0.0 (CallFunction|GetSpawnYaw (LocalVariables|GetSpawnLocation))) "1.000000,1.000000,1.000000") "AdjustIfPossibleButAlwaysSpawn" "MultiplyWithRoot" 0 0)))

(fn GetSpawnLocation
  (bind _box (Variables|Default|GetBox))
  (bind (_origin _boxextent) (Collision|GetComponentBounds _box))
  (return (+ _origin (* _boxextent (* (Math|Random|RandomUnitVector) "0.500000,0.500000,0.000000")))))