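; BP_PistolProjectile is the pistol's bullet, a child projectile that deals damage through its parent class.
; FireProjectile shows the sphere, sets the projectile movement velocity and enables query-only collision.
; ApplyDamage runs the parent logic, then calls DeactivateBullet, which is empty, as are BeginPlay and ResetBullet.
; Disconnected nodes hold unused timed reset, deactivation and bullet-pool return logic.
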(event Custom|FireProjectile
  (params (Velocity :type Vector))
  (Rendering|SetVisibility (Variables|Default|GetSphere) true false)
  (Variables|/Script/Engine.MovementComponent|SetVelocity (Variables|Default|GetProjectileMovement) Velocity)
  (Collision|SetCollisionEnabled (Variables|Default|GetSphere) "QueryOnly"))

(event Custom|DeactivateBullet)

(event Custom|ResetBullet)

(event EventBeginPlay)

(fn ConstructionScript
  (|CallParentFunction))

(fn ApplyDamage
  (params (DamagedActor :type Actor%20Object%20Reference))
  (|CallParentFunction DamagedActor)
  (CallFunction|DeactivateBullet))