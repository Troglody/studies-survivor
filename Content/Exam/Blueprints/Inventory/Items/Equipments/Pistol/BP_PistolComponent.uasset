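; BP_PistolComponent is the pistol equipment component, which fires toward the closest enemy when executed.
; After running the parent logic, Execute gathers every BP_Enemy actor in the level and finds the one nearest the owner.
; It spawns an actor at the owner's location, yawed toward that enemy, with the owning Pawn as Instigator.
; Nothing spawns when no enemies exist or the owner is not a Pawn.
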(fn Execute
  (bind _returnvalue (Components|GetOwner))
  (bind _returnvalue_2 (Transformation|GetActorTransform _returnvalue))
  (|CallParentFunction)
  (bind _outactors (Actor|GetAllActorsOfClass "/Game/Exam/Blueprints/Gameplay/BP_Enemy.BP_Enemy_C"))
  (if (Utilities|Array|IsNotEmpty _outactors)
    (bind _aspawn (Utilities|Casting|CastToPawn (Components|GetOwner)))
    (Game|SpawnActorfromClass "/Game/Exam/Blueprints/Inventory/Items/Equipments/Pistol/BP_PistolProjectile.BP_PistolProjectile_C" (Math|Transform|MakeTransform (.location _returnvalue_2) (Math|Rotator|MakeRotator 0.0 0.0 (.yaw (Math|Rotator|FindLookatRotation (.location _returnvalue_2) (Transformation|GetActorLocation (.ReturnValue (Actor|FindNearestActor (.location _returnvalue_2) _outactors)))))) "1.000000,1.000000,1.000000") "AdjustIfPossibleButAlwaysSpawn" "MultiplyWithRoot" 0 _aspawn)))