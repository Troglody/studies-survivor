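; BP_EquipmentComponent is an equipment component in the inventory item system that fires a repeating interval trigger.
; Tick accumulates delta time in CurrentTime and calls Execute once it reaches TriggerInterval.
; Execute only subtracts the interval, carrying any overshoot into the next cycle, and holds no equipment effect of its own.
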(event EventBeginPlay)

(event EventTick
  (params (DeltaSeconds :type Float%20%28single-precision%29))
  (bind _output_get (Variables|Gameplay|SetCurrentTime (+ (Variables|Gameplay|GetCurrentTime) DeltaSeconds)))
  (if (>= _output_get (Variables|Gameplay|GetTriggerInterval))
    (Gameplay|Execute)))

(fn Execute
  (Variables|Gameplay|SetCurrentTime (- (Variables|Gameplay|GetCurrentTime) (Variables|Gameplay|GetTriggerInterval))))